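; BP_Crystal is a collectable crystal that flies into the player and vanishes when the player overlaps it.
; On overlap it caches its location, scale and point light intensity, then plays CollectionTimeline.
; Separate timeline tracks lerp it toward the player pawn's live location, shrink it to zero scale and fade its light.
; The actor destroys itself when the timeline finishes.
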(event `self.ReceiveActorBeginOverlap`
  (params (OtherActor :type "Actor Object Reference"))
  (`/Game/Blueprints/Libraries/CC_MacroLibrary.IsPlayer` OtherActor
    (:`Is Player`
      (`self.Store Starting Values`)
      (bind (_direction _collection_progress _scale_progress _light_intensity) (`Timeline|Collection Timeline`)
        (:`Update`
          (`self.Move To Player` _collection_progress)
          (`self.Interpolate Size` _scale_progress)
          (`self.Interpolate Light Intensity` _light_intensity))
        (:`Finished`
          (`self.K2_DestroyActor`))))))

(fn `Interpolate Light Intensity`
  (params (Alpha :type "Float (double-precision)"))
  (`LightComponent.SetIntensity` (`self.PointLight`) (`KismetMathLibrary.Lerp` (`self.Lerp Start Intensity`) 0.0 Alpha)))

(fn `Interpolate Size`
  (params (Alpha :type "Float (double-precision)"))
  (`self.SetActorScale3D` (`KismetMathLibrary.VLerp` (`self.Lerp Start Size`) (0.0 0.0 0.0) Alpha)))

(fn `Move To Player`
  (params (Alpha :type "Float (double-precision)"))
  (`self.K2_SetActorLocation` (`KismetMathLibrary.VLerp` (`self.Lerp Start Position`) (`self.K2_GetActorLocation` (`GameplayStatics.GetPlayerPawn` 0)) Alpha)))

(fn `Store Starting Values`
  (set `self.Lerp Start Position` (`self.K2_GetActorLocation`))
  (set `self.Lerp Start Size` (`self.GetActorScale3D`))
  (set `self.Lerp Start Intensity` (`LightComponentBase.Intensity` (`self.PointLight`))))

(fn `UserConstructionScript`)