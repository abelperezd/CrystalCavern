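; BP_Cannon is a cannon actor that fires projectiles automatically and repeatedly from BeginPlay.
; Each cycle waits for FireRate, then spawns a BP_Projectile at the ProjectileSpawnPoint's location and rotation, scaled by ProjectileScale.
; CannonFireTimeline then slides the cannon mesh along its local Y axis for recoil, and its Cannon Fired output loops back to the delay to start the next shot.
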(event `self.ReceiveBeginPlay`
  (`KismetSystemLibrary.Delay` (`self.Fire Rate`) :!label _label)
  (`self.Spawn Projectile`)
  (bind (_direction _cannon_recoil) (`Timeline|Cannon Fire Timeline` :!via `PlayFromStart`)
    (:`Update`
      (`self.Move Cannon` _cannon_recoil))
    (:`Cannon Fired`
      (goto _label))))

(fn `Move Cannon`
  (params (`Cannon Y Location` :type "Float (double-precision)"))
  (`SceneComponent.K2_SetRelativeLocation` (`self.StaticMesh Cannon`) (`KismetMathLibrary.MakeVector` 0.0 `Cannon Y Location`) false false))

(fn `Spawn Projectile`
  (bind _projectile_spawn_point (`self.Projectile Spawn Point`))
  (`|SpawnActorFromClass` "/Game/Blueprints/Actors/Projectiles/BP_Projectile.BP_Projectile_C" (`KismetMathLibrary.MakeTransform` (`SceneComponent.K2_GetComponentLocation` _projectile_spawn_point) (`SceneComponent.K2_GetComponentRotation` _projectile_spawn_point) (`KismetMathLibrary.Conv_DoubleToVector` (`self.Projectile Scale`))) "Undefined" "OverrideRootScale" null null))

(fn `UserConstructionScript`)